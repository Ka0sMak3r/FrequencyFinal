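; Music analyzer actor that plays switchable tracks and turns cooked FFT data into frequency-band levels for UI.
; Each tick it normalizes twelve bands against running maxima, smooths them with envelope attack/release times, applies a floor threshold and averages them into four values.
; A looping timer gates decay of the maxima, so normalization adapts as the music changes.
; Helper functions for band-threshold checks and damage-stack tiers are defined but not called here.
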(event Custom|DecreaseMags
  ;[1 0.7462 0.3521] Sound Analysis
  (Utilities|FlowControl|DoOnce false) ; enters at Reset
)

(event EventTick
  (params (DeltaSeconds :type Float%20%28single-precision%29))
  (Variables|Default|SetDelta%20Seconds DeltaSeconds)
  ;[1 0.7462 0.3521] Sound Analysis
  (Utilities|FlowControl|Sequence
    (:then_0
      (bind _freq2mag (CallFunction|FFTDataFunction))
      (Variables|Default|SetLatestMags _freq2mag))
    (:then_1
      (CallFunction|GetMaxMagnitudes))
    (:then_2
      (CallFunction|NormalizeMagnitudes))
    (:then_3
      (Utilities|FlowControl|Sequence
        (:then_0
          (Utilities|FlowControl|DoOnce false
            (:Completed
              (CallFunction|InitSmoothValues))))
        (:then_1
          (CallFunction|LinearInterpolationFunction))))
    (:then_4
      (CallFunction|LowThreshold))
    (:then_5
      (Utilities|FlowControl|DoOnce false
        (:Completed
          (CallFunction|DecreasePreviousMaxMagnitudes))))
    (:then_7
      (CallFunction|MagnitudeUIvalues))))

(event EventBeginPlay
  (bind _returnvalue (Game|GetPlayerController 0))
  (bind _audio (Variables|Default|GetAudio))
  (bind _new_sound (Variables|Default|GetNew%20Sound))
  (Utilities|FlowControl|Sequence
    (:then_0
      ;[1 0.4654 0.4256] Sound Setter
      (Audio|Components|Audio|SetSound (Variables|Default|GetAudio) _new_sound)
      (Variables|Default|SetDuration (Variables|/Script/Engine.SoundBase|GetDuration _new_sound)))
    (:then_1
      (Variables|Default|SetEnvelope%20Follower%20Attack%20Time (Math|Conversions|ToFloat(Integer) (Variables|/Script/Engine.AudioComponent|GetEnvelopeFollowerAttackTime _audio))))
    (:then_2
      (Variables|Default|SetEnvelope%20Follower%20Release%20Time (Math|Conversions|ToFloat(Integer) (Variables|/Script/Engine.AudioComponent|GetEnvelopeFollowerReleaseTime _audio))))
    (:then_3
      ;[0.2387 1 0.7881] Decreasing Max Magnitudes
      (Actor|Tick|SetActorTickEnabled true))
    (:then_4
      (if true
        (Utilities|Time|SetTimerbyEvent (EventDispatchers|CreateEvent :!event DecreasePreviousMaxMagnitudes) (Variables|Default|GetInterval) true)))
    (:then_5
      ;[0.3889 0.6983 1] Get Player Input
      (Input|EnableInput _returnvalue)
      (Input|SetInputModeGameOnly _returnvalue false))
    (:then_6
      (Variables|Default|SetDamageStack (Variables|Default|GetDamageStack)))))

(event Input|KeyboardEvents|1
  (params (Key :type Key%20Structure :default "None"))
  (bind _audio (Variables|Default|GetAudio))
  ;[0.4244 0.3612 1] Music Playlist
  (:Pressed
    (Audio|Components|Audio|SetSound _audio (Variables|Default|GetTrack1)))
  (:Released
    (Audio|Components|Audio|Play _audio 0.0)))

(event Input|KeyboardEvents|2
  (params (Key :type Key%20Structure :default "None"))
  (bind _audio (Variables|Default|GetAudio))
  ;[0.4244 0.3612 1] Music Playlist
  (:Pressed
    (Audio|Components|Audio|SetSound _audio (Variables|Default|GetTrack2)))
  (:Released
    (Audio|Components|Audio|Play _audio 0.0)))

(fn ConstructionScript)

(fn FFTDataFunction
  ;[1 0.2054 0.1656] Get Magnitude from Input Frequencies
  (bind _outsoundwavespectraldata (Class|AudioComponent|GetCookedFFTData (Variables|Default|GetAudio) (Variables|Default|GetFreqArray)))
  (return (Utilities|Array|MakeArray (.Output_Magnitude (Utilities|FrequencytoMagnitudeMacro _outsoundwavespectraldata)) (.Output_Magnitude2 (Utilities|FrequencytoMagnitudeMacro _outsoundwavespectraldata)) (.Output_Magnitude3 (Utilities|FrequencytoMagnitudeMacro _outsoundwavespectraldata)) (.Output_Magnitude4 (Utilities|FrequencytoMagnitudeMacro _outsoundwavespectraldata)) (.Output_Magnitude5 (Utilities|FrequencytoMagnitudeMacro _outsoundwavespectraldata)) (.Output_Magnitude6 (Utilities|FrequencytoMagnitudeMacro _outsoundwavespectraldata)) (.Output_Magnitude7 (Utilities|FrequencytoMagnitudeMacro _outsoundwavespectraldata)) (.Output_Magnitude8 (Utilities|FrequencytoMagnitudeMacro _outsoundwavespectraldata)) (.Output_Magnitude9 (Utilities|FrequencytoMagnitudeMacro _outsoundwavespectraldata)) (.Output_Magnitude10 (Utilities|FrequencytoMagnitudeMacro _outsoundwavespectraldata)) (.Output_Magnitude11 (Utilities|FrequencytoMagnitudeMacro _outsoundwavespectraldata)) (.Output_Magnitude12 (Utilities|FrequencytoMagnitudeMacro _outsoundwavespectraldata)))))

(fn GetMaxMagnitudes
  ;[1 0.1129 0.3445] Get Max Magnitudes
  (for (_array_element _array_index) (Variables|Default|GetLatestMags)
    (Variables|Default|SetLastestMag _array_element)
    (Variables|Default|SetCurrentIndex _array_index)
    (Utilities|Array|Add (LocalVariables|GetMaxMagLocal) (Math|Float|SelectFloat (Variables|Default|GetLastestMag) (Utilities|Array|Get(acopy) (Variables|Default|GetMaxMagnitudes) (Variables|Default|GetCurrentIndex)) (> (Variables|Default|GetLastestMag) (Utilities|Array|Get(acopy) (Variables|Default|GetMaxMagnitudes) (Variables|Default|GetCurrentIndex))))))
  (Variables|Default|SetMaxMagnitudes (LocalVariables|GetMaxMagLocal)))

(fn NormalizeMagnitudes
  ;[1 0.1758 0.3976] Normalize Magnitudes
  (Variables|Default|SetMaxMagnitude (.MaxValue (Math|Float|MaxOfFloatArray (Variables|Default|GetMaxMagnitudes))))
  (for (_array_element _array_index) (Variables|Default|GetLatestMags)
    (Utilities|Array|Add (LocalVariables|GetNormalizedMagLocal) (Math|Float|MapRangeClamped _array_element 0.0 (Math|Float|SelectFloat (Utilities|Array|Get(acopy) (Variables|Default|GetMaxMagnitudes) _array_index) (Variables|Default|GetMaxMagnitude) (LocalVariables|GetNormalizeEachFreq)) 0.0 1.0)))
  (Variables|Default|SetNormalizedMagnitudes (LocalVariables|GetNormalizedMagLocal)))

(fn InitSmoothValues
  ;[0.6211 0.3417 1] Initialize Smooth Magnitudes
  (for (_ _array_index) (Variables|Default|GetNormalizedMagnitudes)
    (Utilities|Array|SetArrayElem (Variables|Default|GetSmoothMagnitudes) _array_index 0.0 true)))

(fn LinearInterpolationFunction
  ;[1 0.1797 0.4223] Magnitude Smoothing based on Analysis Period
  (for (_array_element _array_index) (Variables|Default|GetNormalizedMagnitudes)
    (Utilities|Array|Add (LocalVariables|GetSmoothMagsLocal) (Math|Interpolation|FInterptoConstant (Utilities|Array|Get(acopy) (Variables|Default|GetSmoothMagnitudes) _array_index) _array_element (Variables|Default|GetDelta%20Seconds) (Math|Float|SelectFloat (/ 1.0 (/ (Variables|Default|GetEnvelope%20Follower%20Attack%20Time) 1e+03)) (/ 1.0 (/ (Variables|Default|GetEnvelope%20Follower%20Release%20Time) 1e+03)) (> _array_element (Utilities|Array|Get(acopy) (Variables|Default|GetSmoothMagnitudes) _array_index))))))
  (Variables|Default|SetSmoothMagnitudes (LocalVariables|GetSmoothMagsLocal)))

(fn DecreasePreviousMaxMagnitudes
  ;[1 0.294 0.2143] Decrease Magnitudes
  (for _array_element (Variables|Default|GetMaxMagnitudes)
    (Utilities|Array|Add (LocalVariables|GetMaxMagnitudesLocal) (Math|Float|Clamp(Float) (* _array_element (Math|Float|MapRangeClamped (Variables|Default|GetAggresiveness) 0.0 1.0 1.0 0.0)) 0.0001 9999.0)))
  (Variables|Default|SetMaxMagnitudes (LocalVariables|GetMaxMagnitudesLocal)))

(fn LowThreshold
  ;[0.2266 1 0.1985] Lowest Threshold of Magnitudes
  (Utilities|Array|Clear (Variables|Default|GetTempStore))
  (for _array_element (Variables|Default|GetSmoothMagnitudes)
    (Utilities|Array|Add (Variables|Default|GetTempStore) (Math|Float|MapRangeClamped _array_element (Variables|Default|GetLowerThreshold) 1.0 0.0 1.0)))
  (bind _output_get (Variables|Default|SetThresholdValues (Variables|Default|GetTempStore)))
  (Variables|Default|SetFinalEnvelopeMagnitudes _output_get))

(fn ThresholdChecker
  (Utilities|FlowControl|Sequence
    (:then_0
      (bind _output_get (LocalVariables|SetBarThresholdA (Math|Float|InRange(Float) (Utilities|Array|Get(acopy) (Variables|Default|GetMagnitudesForUI)) (Variables|Default|GetCusThresholdAmin) (Variables|Default|GetCusThresholdAmax))))
      (bind _output_get_2 (Variables|Default|SetBTA _output_get))
      (if _output_get_2
        (return)))
    (:then_1
      (bind _output_get_3 (LocalVariables|SetBarThresholdB (Math|Float|InRange(Float) (Utilities|Array|Get(acopy) (Variables|Default|GetMagnitudesForUI) 1) (Variables|Default|GetCusThresholdBmin) (Variables|Default|GetCusThresholdBmax))))
      (bind _output_get_4 (Variables|Default|SetBTB _output_get_3))
      (if _output_get_4
        (return)))
    (:then_2
      (bind _output_get_5 (LocalVariables|SetBarThresholdC (Math|Float|InRange(Float) (Utilities|Array|Get(acopy) (Variables|Default|GetMagnitudesForUI) 2) (Variables|Default|GetCusThresholdCmin) (Variables|Default|GetCusThresholdCmax))))
      (bind _output_get_6 (Variables|Default|SetBTC _output_get_5))
      (if _output_get_6
        (return)))
    (:then_3
      (bind _output_get_7 (LocalVariables|SetBarThresholdD (Math|Float|InRange(Float) (Utilities|Array|Get(acopy) (Variables|Default|GetMagnitudesForUI) 3) (Variables|Default|GetCusThresholdDmin) (Variables|Default|GetCusThresholdDmax))))
      (bind _output_get_8 (Variables|Default|SetBTD _output_get_7))
      (if _output_get_8
        (return)))))

(fn MagnitudeUIvalues
  (bind _finalenvelopemagnitudes (Variables|Default|GetFinalEnvelopeMagnitudes))
  (Variables|Default|SetMagnitudesForUI (Utilities|Array|MakeArray (/ (+ (Utilities|Array|Get(acopy) _finalenvelopemagnitudes) (Utilities|Array|Get(acopy) _finalenvelopemagnitudes 1) (Utilities|Array|Get(acopy) _finalenvelopemagnitudes 2)) 3.0) (/ (+ (Utilities|Array|Get(acopy) _finalenvelopemagnitudes 3) (Utilities|Array|Get(acopy) _finalenvelopemagnitudes 4) (Utilities|Array|Get(acopy) _finalenvelopemagnitudes 5)) 3.0) (/ (+ (Utilities|Array|Get(acopy) _finalenvelopemagnitudes 6) (Utilities|Array|Get(acopy) _finalenvelopemagnitudes 7) (Utilities|Array|Get(acopy) _finalenvelopemagnitudes 8)) 3.0) (/ (+ (Utilities|Array|Get(acopy) _finalenvelopemagnitudes 9) (Utilities|Array|Get(acopy) _finalenvelopemagnitudes 10) (Utilities|Array|Get(acopy) _finalenvelopemagnitudes 11)) 3.0))))

(fn StackChecker
  (params (DSIn :type Integer))
  (if (!= DSIn 12)
    (bind _output_get (Variables|Default|SetDamageStack (+ (Variables|Default|GetDamageStack) 1)))
    (Utilities|FlowControl|Sequence
      (:then_0
        (if (== (Variables|Default|GetDamageStack) (Variables|Default|GetMaxStack))
          (Variables|Default|SetStackC true)
          (Variables|Default|SetStackA false)
          (Variables|Default|SetStackB false)
          (return)))
      (:then_1
        (if (>= (Variables|Default|GetDamageStack) 8)
          (Variables|Default|SetStackB true)
          (Variables|Default|SetStackA false)
          (return)))
      (:then_2
        (if (>= _output_get 4)
          (Variables|Default|SetStackA true)
          (return))))))