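; Audio-reactive particle emitter actor that spawns BP_DiscoBox actors as particles, driven by FFT envelope magnitudes from FFTDataRef.
; A timeline started on BeginPlay moves the emitter between two points.
; Tick uses a 0.2-second Delay to pace spawns, giving each box a limited lifespan, acceleration and randomized, magnitude-scaled velocity.
; Each tick also writes the last envelope value to the "Multiplier" material parameter on all boxes' discs.
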(event EventBeginPlay
  ;[0.1603 1 0.3702] Lerping the Particle Emitter location
  (bind _newtrack_0 (Timeline|Timeline PlayFromStart)
    (:Update
      (Transformation|SetActorLocation (Math|Vector|Lerp(Vector) (Variables|Default|GetA) (Variables|Default|GetB) _newtrack_0) false false))))

(event EventTick
  (params (DeltaSeconds :type Float%20%28single-precision%29))
  (Utilities|FlowControl|Sequence
    (:then_0
      (Variables|Default|SetFinal%20Envelope%20MagnitudesHere (Variables|/Game/Blueprints/SoundAnalyzers/BP_FFTData.BP_FFTData_C|GetFinalEnvelopeMagnitudes (Variables|Default|GetFFTDataRef))))
    (:then_1
      ;[1 0.04167 0.04167] Particle Emitter Logic
      (Utilities|FlowControl|Delay 0.2)
      (bind _returnvalue (Game|SpawnActorfromClass "/Game/Blueprints/ParticleSystem/BP_DiscoBox.BP_DiscoBox_C" (Transformation|GetActorTransform) "Undefined" 0 0))
      (Actor|SetLifeSpan _returnvalue 2e+01)
      (Variables|/Game/Blueprints/ParticleSystem/BP_DiscoBox.BP_DiscoBox_C|SetAcc _returnvalue (Math|Vector|MakeVector 8e+01 -8e+01 1e+02))
      (Variables|/Game/Blueprints/ParticleSystem/BP_DiscoBox.BP_DiscoBox_C|SetVelocity _returnvalue (+ (* (Math|Random|RandomUnitVector) (Math|Vector|MakeVector (* (Math|Random|RandomFloatinRange -7.0 -8.0) 1e+02) (* (Math|Random|RandomFloatinRange 7.0 8.0) 1e+02) (* (stale _array_element) 1e+03))) (* (* (stale _array_element) 1e+03) (Math|Random|RandomUnitVector)))))
    (:then_2
      ;[1 0.7021 0.2891] Setting the Velocity Using the Magnitude values
      (for _array_element (Variables|Default|GetFinal%20Envelope%20MagnitudesHere)
        (Variables|Default|SetEnvelopeInputForMaterial _array_element)))
    (:then_3
      (bind _outactors (Actor|GetAllActorsOfClass "/Game/Blueprints/ParticleSystem/BP_DiscoBox.BP_DiscoBox_C"))
      (Variables|Default|SetOut%20ActorsHere _outactors))
    (:then_4
      ;[0.11 0.1482 1] Setting Values to the Particle Material
      (for _array_element_2 (Variables|Default|GetOut%20ActorsHere)
        (Rendering|Material|SetMaterial (Variables|/Game/Blueprints/ParticleSystem/BP_DiscoBox.BP_DiscoBox_C|GetDisc _array_element_2) 0 (Rendering|Material|GetMaterial (Variables|/Game/Blueprints/ParticleSystem/BP_DiscoBox.BP_DiscoBox_C|GetDisc _array_element_2) 0))
        (Rendering|Material|SetScalarParameterValueonMaterials (Variables|/Game/Blueprints/ParticleSystem/BP_DiscoBox.BP_DiscoBox_C|GetDisc _array_element_2) "Multiplier" (Variables|Default|GetEnvelopeInputForMaterial))))))

(fn ConstructionScript)