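; BP_Temp1 is a spawner for audio-reactive visualizers, creating a row of twelve BP_VisualizerB actors along Y on BeginPlay.
; Each Tick it reads envelope magnitudes and duration from FFTDataRef and reapplies AudioReactive_Mat to every visualizer's plane.
; The same loop writes each Pi-scaled magnitude and the duration to shared BP_MaterialParam collection parameters, so each iteration overwrites the previous value.
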(event EventBeginPlay
  (bind _defaultsceneroot (Variables|Default|GetDefaultSceneRoot))
  (bind _returnvalue (Transformation|GetWorldLocation _defaultsceneroot))
  ;[1 0.1284 0.4876] Spawn Audio Reactive Material
  (for _index (range 1 12)
    (Game|SpawnActorfromClass "/Game/Blueprints/Visualizers/BP_VisualizerB.BP_VisualizerB_C" (Math|Transform|MakeTransform (Math|Vector|MakeVector (.x _returnvalue) (+ (.y _returnvalue) (* _index 800)) (.z _returnvalue)) "0, 0, 0" "1.000000,1.000000,1.000000") "Undefined" 0 0))
  (bind _outactors (Actor|GetAllActorsOfClass "/Game/Blueprints/Visualizers/BP_VisualizerB.BP_VisualizerB_C"))
  (Variables|Default|SetOut%20Actors _outactors))

(event EventTick
  (params (DeltaSeconds :type Float%20%28single-precision%29))
  (bind _fftdataref (Variables|Default|GetFFTDataRef))
  (Utilities|FlowControl|Sequence
    (:then_0
      (Variables|Default|SetFinal%20Envelope%20MagnitudesHere (Variables|/Game/Blueprints/SoundAnalyzers/BP_FFTData.BP_FFTData_C|GetFinalEnvelopeMagnitudes _fftdataref)))
    (:then_1
      ;[0.3203 0.1892 1] Passing Parameters to Audio Reactive Material
      (for (_array_element _array_index) (Variables|Default|GetOut%20Actors)
        (Rendering|Material|SetMaterial (Variables|/Game/Blueprints/Visualizers/BP_VisualizerB.BP_VisualizerB_C|GetPlane _array_element) 0 "/Game/Material/AudioReactive_Mat.AudioReactive_Mat")
        (Rendering|Material|SetScalarParameterValue "/Game/Material/BP_MaterialParam.BP_MaterialParam" "Scalar" (Math|Float|MultiplybyPi (Utilities|Array|Get(acopy) (Variables|Default|GetFinal%20Envelope%20MagnitudesHere) _array_index)) :!class /Script/Engine.KismetMaterialLibrary)
        (Rendering|Material|SetScalarParameterValue "/Game/Material/BP_MaterialParam.BP_MaterialParam" "MusicDuration" (Variables|Default|GetDurationHere) :!class /Script/Engine.KismetMaterialLibrary)))
    (:then_2
      (Variables|Default|SetDurationHere (Variables|/Game/Blueprints/SoundAnalyzers/BP_FFTData.BP_FFTData_C|GetDuration _fftdataref)))))

(fn ConstructionScript)