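; BP_Temp2 is a template waveform spawner that turns FFT envelope magnitudes into BP_VisualizerA actors.
; On Tick it loops over the cached magnitudes, then refreshes that cache from FFTDataRef.
; The spawn transform offsets along Y by array index from the root and scales Z by magnitude.
; A latent Delay inside the loop precedes the spawn, so iterations do not each produce their own actor.
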(event EventTick
  (params (DeltaSeconds :type Float%20%28single-precision%29))
  (bind _defaultsceneroot (Variables|Default|GetDefaultSceneRoot))
  (bind _returnvalue (Transformation|GetWorldLocation _defaultsceneroot))
  ;[0.2633 0.4615 1] WaveForm Spawner
  (Utilities|FlowControl|Sequence
    (:then_0
      (for (_array_element _array_index) (Variables|Default|GetFinal%20Envelope%20MagnitudesHere)
        (Utilities|FlowControl|Delay 0.01)
        (Game|SpawnActorfromClass "/Game/Blueprints/Visualizers/BP_VisualizerA.BP_VisualizerA_C" (Math|Transform|MakeTransform (Math|Vector|MakeVector (.x _returnvalue) (+ (.y _returnvalue) (* _array_index 100)) (.z _returnvalue)) "0, 0, 0" (Math|Vector|MakeVector 1.0 1.0 (* _array_element 1e+01))) "Undefined" 0 0)))
    (:then_1
      (Variables|Default|SetFinal%20Envelope%20MagnitudesHere (Variables|/Game/Blueprints/SoundAnalyzers/BP_FFTData.BP_FFTData_C|GetFinalEnvelopeMagnitudes (Variables|Default|GetFFTDataRef))))))

(fn ConstructionScript)