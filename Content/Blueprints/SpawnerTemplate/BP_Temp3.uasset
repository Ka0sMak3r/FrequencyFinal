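; BP_Temp3 is an audio visualizer spawner that builds a row of band actors and scales them with FFT magnitudes.
; On BeginPlay it spawns BP_VisualizerC actors along world Y, then caches every actor of that class.
; Each Tick sets their Z scale from the envelope magnitude at the matching index plus a minimum.
; Magnitudes refresh from FFTDataRef after scaling, so bars use the previous tick's data.
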(event EventBeginPlay
  (bind _defaultsceneroot (Variables|Default|GetDefaultSceneRoot))
  (bind _returnvalue (Transformation|GetWorldLocation _defaultsceneroot))
  ;[0.008226 1 0.4045] Spawn Normal Bands
  (for _index (range 1 12)
    (Game|SpawnActorfromClass "/Game/Blueprints/Visualizers/BP_VisualizerC.BP_VisualizerC_C" (Math|Transform|MakeTransform (Math|Vector|MakeVector (.x _returnvalue) (+ (.y _returnvalue) (* _index 700)) (.z _returnvalue)) "0, 0, 0" "1.000000,1.000000,1.000000") "Undefined" 0 0))
  (bind _outactors (Actor|GetAllActorsOfClass "/Game/Blueprints/Visualizers/BP_VisualizerC.BP_VisualizerC_C"))
  (Variables|Default|SetOut%20Actors _outactors))

(event EventTick
  (params (DeltaSeconds :type Float%20%28single-precision%29))
  (Utilities|FlowControl|Sequence
    (:then_0
      ;[1 0.9109 0.1354] Scale Normal Bands
      (for (_array_element _array_index) (Variables|Default|GetOut%20Actors)
        (Transformation|SetRelativeScale3D (Variables|/Game/Blueprints/Visualizers/BP_VisualizerC.BP_VisualizerC_C|GetScene _array_element) (Math|Vector|MakeVector 2.0 2.0 (+ (* (Utilities|Array|Get(acopy) (Variables|Default|GetFinal%20Envelope%20MagnitudesHere) _array_index) 1e+01) (Variables|Default|GetMinScale))))))
    (:then_1
      (Variables|Default|SetFinal%20Envelope%20MagnitudesHere (Variables|/Game/Blueprints/SoundAnalyzers/BP_FFTData.BP_FFTData_C|GetFinalEnvelopeMagnitudes (Variables|Default|GetFFTDataRef))))))

(fn ConstructionScript)